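; BP_Luz2 is a light Blueprint whose PointLight switches on and off in response to external events.
; On BeginPlay it hides the light and binds its handlers to the DarLuz and ApagarLuz dispatchers on Delegado.
; Both handlers call the same toggle, which flips Prendido and applies it as the light's visibility, so neither dispatcher forces a specific on or off state.
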(event `apagarluz`
  (`self.ejecutarencendido`))

(event `self.ReceiveBeginPlay`
  (bind _delegado (`self.Delegado`))
  (set `self.Prendido` false)
  (`SceneComponent.SetVisibility` (`self.PointLight`) false false)
  (add `/Game/Blueprints/LUZ/prueba/BP_ELSWITCH.darLuz` _delegado (delegate `RecibirLuz`))
  (add `/Game/Blueprints/LUZ/prueba/BP_ELSWITCH.apagarluz` _delegado (delegate `apagarluz`)))

(event `RecibirLuz`
  (`self.ejecutarencendido`))

(event `ejecutarencendido`
  (bind _output_get (set `self.Prendido` (not (`self.Prendido`))))
  (`SceneComponent.SetVisibility` (`self.PointLight`) _output_get false))

(fn `UserConstructionScript`)