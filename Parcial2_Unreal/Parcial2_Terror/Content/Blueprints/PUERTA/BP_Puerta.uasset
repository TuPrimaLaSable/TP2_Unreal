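; Interactable door Blueprint that toggles between open and closed each time its Interactuable event fires.
; AnimacionPuerta flips EstaAbierta and plays a 2D sound: a door slam when switching to open, a creak when switching to closed.
; The flipped state plays or reverses TL_Abrirpuerta, whose track drives a rotator lerp that swings the Pivote component through 90 degrees.
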(event `/Game/Blueprints/Interface/BPI_Interactor.Interactuable`
  (`self.AnimacionPuerta` (`self.estaAbierta`))
  (if (`self.estaAbierta`)
    (bind (_direction _newtrack_0) (`Timeline|TL_Abrirpuerta` :!via `Reverse` :!label _label)
      (:`Update`
        (`SceneComponent.K2_SetRelativeRotation` (`self.pivote`) (`KismetMathLibrary.RLerp` (struct) (struct :`Yaw` 90.0) _newtrack_0) false false)))
    (else
      (goto _label))))

(event `self.ReceiveTick`
  (params (DeltaSeconds :type "Float (single-precision)")))

(event `self.ReceiveBeginPlay`)

(fn `AnimacionPuerta`
  (params (ValorPuerta :type Boolean))
  (if ValorPuerta
    (set `self.estaAbierta` false)
    (`GameplayStatics.SpawnSound2D` "/Game/Blueprints/PUERTA/dragon-studio-creaky-old-door-472357.dragon-studio-creaky-old-door-472357" 1.0 1.0 0.0 null)
    (else
      (set `self.estaAbierta` true)
      (`GameplayStatics.SpawnSound2D` "/Game/Blueprints/PUERTA/freesound_community-wood-door-slam-46791.freesound_community-wood-door-slam-46791" 1.0 1.0 0.0 null))))

(fn `UserConstructionScript`)